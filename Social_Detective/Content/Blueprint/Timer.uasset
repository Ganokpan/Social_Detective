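; Timer actor that shows a Countdown_UI widget on screen at BeginPlay and runs a minutes and seconds counter.
; Tick feeds a one-second Delay that paces the counter update.
; Each update sets Minutes to Second plus one, then bumps Minutes and resets Second when Second exceeds 59.
; Second is never incremented in this graph, and the values are not passed to the widget here.
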(event EventBeginPlay
  (bind _returnvalue (UserInterface|CreateWidget "/Game/UI/Countdown_UI.Countdown_UI_C"))
  (UserInterface|Viewport|AddtoViewport _returnvalue 0))

(event EventTick
  (params (DeltaSeconds :type Float%20%28single-precision%29))
  (Utilities|FlowControl|Delay 1.0)
  (Variables|Default|SetMinutes (+ (Variables|Default|GetSecond) 1))
  (if (> (Variables|Default|GetSecond) 59)
    (Variables|Default|SetMinutes (+ (Variables|Default|GetMinutes) 1))
    (Variables|Default|SetSecond 0)))

(fn ConstructionScript)