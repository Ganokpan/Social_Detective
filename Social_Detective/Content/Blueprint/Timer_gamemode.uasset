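; Game mode that runs a countdown timer and shows it through a Countdown_UI widget created on BeginPlay.
; Tick feeds a one-second Delay, so Second drops by one roughly every second until it reaches zero.
; Minutes is always set to 0, and the node that would decrement it is left unconnected.
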(event EventBeginPlay
  (bind _returnvalue (UserInterface|CreateWidget "/Game/UI/Countdown_UI.Countdown_UI_C"))
  (UserInterface|Viewport|AddtoViewport _returnvalue 0))

(event EventTick
  (params (DeltaSeconds :type Float%20%28single-precision%29))
  (Utilities|FlowControl|Delay 1.0)
  (Variables|Default|SetMinutes 0)
  (if (> (Variables|Default|GetSecond) 0)
    (Variables|Default|Setsecond (- (Variables|Default|Getsecond) 1))
    (Variables|Default|SetMinutes 0)))

(fn ConstructionScript)