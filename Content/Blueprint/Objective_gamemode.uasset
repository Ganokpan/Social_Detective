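; Objective game mode, by its name, that puts a countdown widget on screen when play begins.
; Every tick it tries to cast its owner to Clue1; on success it sets a Clue1 counter to zero and adds zero to it.
; The objective tracking looks unfinished: the counter never rises and the clue's Found value is left unused.
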(event EventBeginPlay
  (bind _returnvalue (UserInterface|CreateWidget "/Game/UI/Countdown_UI.Countdown_UI_C"))
  (UserInterface|Viewport|AddtoViewport _returnvalue 0))

(event EventTick
  (params (DeltaSeconds :type Float%20%28single-precision%29))
  (bind _asclue_1 (Utilities|Casting|CastToClue1 (Components|GetOwner)))
  (Variables|Default|SetClue_1 0)
  (if (== (Variables|Default|GetClue_1) 0)
    (Variables|Default|SetClue_1 (+ 0 (Variables|Default|GetClue_1)))))

(fn ConstructionScript)